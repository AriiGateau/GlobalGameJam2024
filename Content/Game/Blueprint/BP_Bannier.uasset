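; BP_Bannier is a banner actor that displays the player BP_Bouffon's random combo on a randomly chosen side.
; BeginCombo plays the left or right banner montage, then spawns a vertical column of BP_ComboUnit actors from RandomCombo and plays a curtain sound on the matching side.
; When the montage blends out, it destroys the spawned units and clears their array.
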(event `self.ReceiveBeginPlay`
  ;[1 1 1] Set Initial Variable
  (bind _asbp_bouffon (cast `/Game/Game/Blueprint/BP_Bouffon` (`GameplayStatics.GetPlayerCharacter` 0)))
  (set `self.BP_Bouffon` _asbp_bouffon))

(event `BeginCombo`
  (bind _randombool (`self.RandomBool`))
  (bind _child (`self.Child`))
  (set `self.Index` 0)
  (set `self.RandomBool` (`KismetMathLibrary.RandomBool`))
  (`|PlayMontage` (select `bool` _randombool :`false` (`self.SkeletalMeshGauche`) :`true` (`self.SkeletalMeshDroite`)) (select `bool` _randombool :`false` "/Game/Game/Props/Bannier/AM_BaniereGauche.AM_BaniereGauche" :`true` "/Game/Game/Props/Bannier/AM_BaniereDroite.AM_BaniereDroite" :!type "AnimMontage Object Reference")
    (:`then`
      (`self.SpawnComboUnit`)
      (`GameplayStatics.PlaySoundAtLocation` "/Game/Game/Sound/Bannier/A_Curtain_Cue.A_Curtain_Cue" (`KismetMathLibrary.MakeVector` (`KismetMathLibrary.SelectFloat` 600.0 -600.0 (`self.RandomBool`))) (struct) 1.0 1.0 0.0 null null null null))
    (:`OnBlendOut`
      (for _array_element _child
        (`/Engine/EditorBlueprintResources/StandardMacros.IsValid` _array_element
          (:`Is Valid`
            (`self.K2_DestroyActor` _array_element))))
      (`KismetArrayLibrary.Array_Clear` _child))))

(event `SpawnComboUnit`
  (for (_array_element _array_index) (`/Game/Game/Blueprint/BP_Bouffon.RandomCombo` (`self.BP_Bouffon`))
    (bind _returnvalue (`|SpawnActorFromClass` "/Game/Game/Blueprint/BP_ComboUnit.BP_ComboUnit_C" (`KismetMathLibrary.MakeTransform` (`KismetMathLibrary.MakeVector` (select `bool` (`self.RandomBool`) :`false` -330.0 :`true` 1080.0) -590.0 (- 1050.0 (* _array_index 80)))) "Undefined" "MultiplyWithRoot" null _array_element 0.0 null))
    (`KismetArrayLibrary.Array_Add` (`self.Child`) _returnvalue)))

(fn `UserConstructionScript`)