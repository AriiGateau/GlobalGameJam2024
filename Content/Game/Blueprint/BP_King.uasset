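; BP_King is the king actor that presents the jester's (BP_Bouffon) random combo to the player, by talking or by signing.
; KingTalk plays a talk montage, clears old BP_ComboUnit actors and spawns a row of new ones, one per combo entry, which DeleteChild then hides in sequence.
; KingSign steps through the same combo recursively, chaining a left, down, right or up montage with a neutral pose through Blend Out callbacks.
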(event `self.ReceiveBeginPlay`
  ;[1 1 1] Set Initial Variable
  (bind _asbp_bouffon (cast `/Game/Game/Blueprint/BP_Bouffon` (`GameplayStatics.GetPlayerCharacter` 0)))
  (set `self.BP_Bouffon` _asbp_bouffon))

(event `KingTalk`
  ;[1 1 1] Spawn Combo As Button
  (`|PlayMontage` (`self.King`) "/Game/Game/Props/King/Anim/AM_Roi_Talk.AM_Roi_Talk"
    (:`then`
      (`self.NukeChildren`)
      (`KismetArrayLibrary.Array_Clear` (`self.Child`))
      (set `self.IndexTalk` 0)
      (set `self.bIsSpawning` true)
      (for (_array_element _array_index) (`/Game/Game/Blueprint/BP_Bouffon.RandomCombo` (`self.BP_Bouffon`))
        (bind _returnvalue (`|SpawnActorFromClass` "/Game/Game/Blueprint/BP_ComboUnit.BP_ComboUnit_C" (`KismetMathLibrary.MakeTransform` (`KismetMathLibrary.MakeVector_NetQuantize` (`KismetMathLibrary.Conv_IntToDouble` (+ (* _array_index 100) -400)) 0.0 650.0)) "Undefined" "MultiplyWithRoot" null _array_element null))
        (`KismetArrayLibrary.Array_Add` (`self.Child`) _returnvalue))
      (set `self.bIsSpawning` false)
      (`KismetSystemLibrary.Delay` 1.0)
      (`self.DeleteChild`))))

(event `NukeChildren`
  ;[1 1 1] Spawn Combo As Button
  (set `self.bIsSpawning` true)
  (bind _outactors (`GameplayStatics.GetAllActorsOfClass` "/Game/Game/Blueprint/BP_ComboUnit.BP_ComboUnit_C"))
  (for _array_element _outactors
    (`self.K2_DestroyActor` _array_element)))

(event `DeleteChild`
  (bind _indextalk (`self.IndexTalk`))
  (bind _child (`self.Child`))
  (bind _output (`|GetArrayItem` _child (`self.IndexTalk`)))
  ;[1 1 1] Delete Each one at a time
  (if (not (`self.bIsSpawning`))
    (`/Engine/EditorBlueprintResources/StandardMacros.IsValid` _output
      (:`Is Valid`
        (`SceneComponent.SetVisibility` (`/Game/Game/Blueprint/BP_ComboUnit.Cylinder` _output) false false)
        (if (== _indextalk (- (`KismetArrayLibrary.Array_Length` _child) 1))
          (set `self.IndexTalk` 0)
          (`KismetArrayLibrary.Array_Clear` (`self.Child`))
          (else
            (`/Engine/EditorBlueprintResources/StandardMacros.IncrementInt` _indextalk
              (:`  `
                (`KismetSystemLibrary.Delay` 0.4)
                (`self.DeleteChild`)))))))))

(event `KingSign`
  (set `self.IndexSign` 0)
  (`self.Direction`))

(event `Direction`
  (bind _indexsign (`self.IndexSign`))
  (bind _king (`self.King`))
  (bind _king_2 (`self.King`))
  (switch `int` (`|GetArrayItem` (`/Game/Game/Blueprint/BP_Bouffon.RandomCombo` (`self.BP_Bouffon`)) (`self.IndexSign`))
    (:`1`
      (`|PlayMontage` _king "/Game/Game/Props/King/Anim/AM_King_Direction_Left.AM_King_Direction_Left" 0.5
        (:`OnBlendOut`
          _)))
    (:`2`
      (`|PlayMontage` _king "/Game/Game/Props/King/Anim/AM_King_Direction_Down.AM_King_Direction_Down" 0.5
        (:`OnBlendOut`
          _)))
    (:`3`
      (`|PlayMontage` _king_2 "/Game/Game/Props/King/Anim/AM_King_Direction_Right.AM_King_Direction_Right" 0.5
        (:`OnBlendOut`
          _)))
    (:`4`
      (`|PlayMontage` _king_2 "/Game/Game/Props/King/Anim/AM_King_Direction_Up.AM_King_Direction_Up" 0.5
        (:`OnBlendOut`
          _))))
  (`KismetSystemLibrary.Delay` 0.2)
  (`|PlayMontage` (`self.King`) "/Game/Game/Props/King/Anim/AM_King_Direction_Neutral.AM_King_Direction_Neutral" 0.8
    (:`OnBlendOut`
      (if (== (- (`KismetArrayLibrary.Array_Length` (`/Game/Game/Blueprint/BP_Bouffon.RandomCombo` (`self.BP_Bouffon`))) 1) _indexsign)
        (set `self.IndexSign` 0)
        (else
          (`/Engine/EditorBlueprintResources/StandardMacros.IncrementInt` _indexsign
            (:`  `
              (`self.Direction`))))))))

(fn `UserConstructionScript`)