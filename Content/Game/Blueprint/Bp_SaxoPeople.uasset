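; Saxophone performer actor that slides onto the stage and acts out the player BP_Bouffon's RandomCombo as directional moves.
; BeginCombo runs a Move timeline along X, then Direction maps each combo entry to left, down, right or up.
; Rotate timeline shifts the actor, adding pitch for up/down only, and RotateBack restores it before the next entry.
; After the last entry, Retreat reverses Move to slide it back.
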(event `self.ReceiveBeginPlay`
  ;[1 1 1] Set Initial Variable
  (set `self.InitialRotation` (`self.K2_GetActorRotation`))
  (set `self.InitialLocation` (`self.K2_GetActorLocation`))
  (bind _asbp_bouffon (cast `/Game/Game/Blueprint/BP_Bouffon` (`GameplayStatics.GetPlayerCharacter` 0)))
  (set `self.BP_Bouffon` _asbp_bouffon))

(event `Start`
  ;[1 1 1] Move The Saxo People In The Stage
  (set `self.bIsFinishPlaying` false)
  (`TimelineComponent.SetPlayRate` (`self.Move`) 3.0)
  (bind (_direction _alpha) (`Timeline|Move` :!via `PlayFromStart` :!label _label)
    (:`Update`
      (`self.K2_SetActorLocation` (`|EaseFunction` "Linear" _alpha (`self.InitialLocation`) (`KismetMathLibrary.MakeVector` (- (.x (`self.InitialLocation`)) (`self.Distance`)) (.y (`self.InitialLocation`)) (.z (`self.InitialLocation`))))))
    (:`Finished`
      (if (not (`self.bIsFinishPlaying`))
        (`KismetSystemLibrary.Delay` 0.2)
        (`self.Direction`)))))

(event `Retreat`
  ;[1 1 1] Move The Saxo People In The Stage
  (set `self.bIsFinishPlaying` true)
  (goto _label :!via `ReverseFromEnd`))

(event `BeginCombo`
  ;[1 1 1] Launch The SaxoPeople
  (set `self.CurrentIndex` 0)
  (`self.Start`))

(event `Direction`
  ;[1 1 1] Determine Which Direction The SaxoPeople Will Play
  (switch `int` (`|GetArrayItem` (`/Game/Game/Blueprint/BP_Bouffon.RandomCombo` (`self.BP_Bouffon`)) (`self.CurrentIndex`))
    (:`1`
      (`self.LeftDirection`))
    (:`2`
      (`self.DownDirection`))
    (:`3`
      (`self.RightDirection`))
    (:`4`
      (`self.UpDirection`))))

(event `ResetLocRot`
  (bind _currentindex (`self.CurrentIndex`))
  ;[1 1 1] Reset To Initial Totation
  (`TimelineComponent.SetPlayRate` (`self.RotateBack`) 8.0)
  (set `self.CurrentRot` (`self.K2_GetActorRotation`))
  (set `self.ModifieLocation` (`self.K2_GetActorLocation`))
  (bind (_direction _alpha) (`Timeline|RotateBack` :!via `PlayFromStart`)
    (:`Update`
      (`self.K2_SetActorRotation` (`|EaseFunction` "Linear" _alpha (`self.CurrentRot`) (`self.InitialRotation`)))
      (`self.K2_SetActorLocation` (`|EaseFunction` "Linear" _alpha (`self.ModifieLocation`) (`self.CurrentLocation`))))
    (:`Finished`
      (if (== (- (`KismetArrayLibrary.Array_Length` (`/Game/Game/Blueprint/BP_Bouffon.RandomCombo` (`self.BP_Bouffon`))) 1) _currentindex)
        (set `self.CurrentIndex` 0)
        (`KismetSystemLibrary.Delay` 0.5)
        (`self.Retreat`)
        (else
          (`/Engine/EditorBlueprintResources/StandardMacros.IncrementInt` _currentindex
            (:`  `
              (`self.Direction`))))))))

(event `LeftDirection`
  ;[1 1 1] Define Direction
  (set `self.DegreeLeftRight` (* (`KismetMathLibrary.Abs` (`self.DegreeLeftRight`)) -1.0))
  (set `self.bIsSide` true)
  (`self.Transition`))

(event `UpDirection`
  ;[1 1 1] Define Direction
  (set `self.DegreeUpDown` (* (`KismetMathLibrary.Abs` (`self.DegreeLeftRight`)) -1.0))
  (set `self.bIsSide` false)
  (`self.Transition`))

(event `RightDirection`
  ;[1 1 1] Define Direction
  (set `self.DegreeLeftRight` (`KismetMathLibrary.Abs` (`self.DegreeLeftRight`)))
  (set `self.bIsSide` true)
  (`self.Transition`))

(event `DownDirection`
  ;[1 1 1] Define Direction
  (set `self.DegreeUpDown` (`KismetMathLibrary.Abs` (`self.DegreeLeftRight`)))
  (set `self.bIsSide` false)
  (`self.Transition`))

(event `Transition`
  (bind _initialrotation (`self.InitialRotation`))
  ;[1 1 1] Change Rotation With Transition
  (set `self.CurrentLocation` (`self.K2_GetActorLocation`))
  (`TimelineComponent.SetPlayRate` (`self.Rotate`) 3.3)
  (bind (_direction _alpha) (`Timeline|Rotate` :!via `PlayFromStart`)
    (:`Update`
      (`self.K2_SetActorLocation` (select `bool` (`self.bIsSide`) :`false` (`|EaseFunction` "Linear" _alpha (`self.CurrentLocation`) (`KismetMathLibrary.MakeVector` (.x (`self.CurrentLocation`)) (.y (`self.CurrentLocation`)) (- (.z (`self.CurrentLocation`)) (`self.DegreeUpDown`)))) :`true` (`|EaseFunction` "Linear" _alpha (`self.CurrentLocation`) (`KismetMathLibrary.MakeVector` (+ (.x (`self.CurrentLocation`)) (`self.DegreeLeftRight`)) (.y (`self.CurrentLocation`)) (.z (`self.CurrentLocation`))))))
      (if (not (`self.bIsSide`))
        (`self.K2_SetActorRotation` (`|EaseFunction` "Linear" _alpha _initialrotation (`KismetMathLibrary.MakeRotator` (.roll _initialrotation) (/ (`self.DegreeUpDown`) 5.0) (.yaw _initialrotation))))))
    (:`Finished`
      (`self.ResetLocRot`))))

(fn `UserConstructionScript`)