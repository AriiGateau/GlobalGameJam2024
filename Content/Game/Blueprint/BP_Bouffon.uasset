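; BP_Bouffon is the player jester and game loop for a timed combo-matching game performed before a king.
; Four inputs play montages and are checked against a random sequence, cued by a weighted-random presenter (king, banner, sax people, god hand) after tutorial rounds.
; Results adjust timer and score; streaks raise difficulty, lengthening combos and speeding time dilation and music pitch.
; It also drives curtain, menus and physical-animation ragdoll on the mesh.
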(event `SetRagdol`
  (bind _bone1 (`self.Bone1`))
  (bind _physicalanimation (`self.PhysicalAnimation`))
  (bind _mesh (`self.Mesh`))
  (bind _bone2 (`self.Bone2`))
  ;[1 1 1] Set Ragdol
  (`PhysicalAnimationComponent.SetSkeletalMeshComponent` _physicalanimation _mesh)
  (`PhysicalAnimationComponent.ApplyPhysicalAnimationSettingsBelow` _physicalanimation _bone1 (make `PhysicalAnimationData` true 200.0) false)
  (`SkeletalMeshComponent.SetAllBodiesBelowSimulatePhysics` _mesh _bone1 true false)
  (`PhysicalAnimationComponent.ApplyPhysicalAnimationSettingsBelow` (`self.PhysicalAnimation`) _bone2 (make `PhysicalAnimationData` true 500.0) true)
  (`SkeletalMeshComponent.SetAllBodiesBelowSimulatePhysics` _mesh _bone2 true true))

(event `self.ReceiveBeginPlay`
  ;[1 1 1] Set up Input Mapping
  (bind _aspc_bouffon (cast `/Game/Game/Core/PC_Bouffon` (`self.GetController`)))
  (bind _returnvalue (pcsubsystem `EnhancedInputLocalPlayerSubsystem` _aspc_bouffon))
  (`/Engine/EditorBlueprintResources/StandardMacros.IsValid` _returnvalue
    (:`Is Valid`
      (`EnhancedInputSubsystemInterface.AddMappingContext` _returnvalue "/Game/Game/Blueprint/Input/IMC_Default.IMC_Default" 0 (struct))
      (`self.SetVariable`))))

(event `PlayAnimSound`
  (`GameplayStatics.PlaySoundAtLocation` (`|GetArrayItem` (`self.AnimSound`) (`self.InputIndex`)) (600.0 0.0 0.0) (struct) 1.0 1.0 0.0 null null null null))

(event `CameraShake`
  (`GameplayStatics.PlayWorldCameraShake` "/Game/Game/Blueprint/BP_Shake.BP_Shake_C" (`self.K2_GetActorLocation`) 100.0 6000.0))

(event `SetVariable`
  (`self.SetRagdol`)
  (`|ExecutionSequence`
    (:`then_0`
      (bind _returnvalue (`GameplayStatics.GetActorOfClass` "/Game/Game/Blueprint/Bp_SaxoPeople.Bp_SaxoPeople_C"))
      (set `self.BP_SaxoPeople` _returnvalue))
    (:`then_1`
      (bind _returnvalue_2 (`GameplayStatics.GetActorOfClass` "/Game/Game/Blueprint/BP_GodHand.BP_GodHand_C"))
      (set `self.BP_GodHand` _returnvalue_2))
    (:`then_2`
      (bind _returnvalue_3 (`GameplayStatics.GetActorOfClass` "/Game/Game/Blueprint/BP_King.BP_King_C"))
      (set `self.BP_King` _returnvalue_3))
    (:`then_3`
      (bind _returnvalue_4 (`GameplayStatics.GetActorOfClass` "/Game/Game/Blueprint/BP_Bannier.BP_Bannier_C"))
      (set `self.BP_Bannier` _returnvalue_4))
    (:`then_4`
      (bind _returnvalue_5 (`GameplayStatics.GetActorOfClass` "/Game/Game/Blueprint/BP_Curtain.BP_Curtain_C"))
      (set `self.BP_Curtain` _returnvalue_5))
    (:`then_5`
      (`KismetSystemLibrary.Delay` 0.2)
      (bind _returnvalue_6 (`|CreateWidget` "/Game/Game/UI/WBP_MainMenu.WBP_MainMenu_C" null self))
      (`UserWidget.AddToViewport` _returnvalue_6 0))))

(event `EnhancedInput|/Game/Game/Blueprint/Input/Actions/IA_Left_Square`
  (params (ActionValue :type Boolean) (ElapsedSeconds :type "Float (double-precision)") (TriggeredSeconds :type "Float (double-precision)") (InputAction :type "InputAction Object Reference" :default "/Game/Game/Blueprint/Input/Actions/IA_Left_Square.IA_Left_Square"))
  ;[1 1 1] Input
  (:`Started`
    (`self.PlayAnimMontage` "/Game/Game/Blueprint/Mesh/Animation/AM_Left.AM_Left")
    (set `self.InputIndex` 1)
    (`self.PlayAnimSound`)
    (if (not (`self.bIsInputBlock`))
      (`KismetArrayLibrary.Array_Add` (`self.CurrentFigurePlay`) (`self.InputIndex`) :!label _label)
      (`self.CheckCombo`)
      (`self.CameraShake`))))

(event `EnhancedInput|/Game/Game/Blueprint/Input/Actions/IA_Down_Cross`
  (params (ActionValue :type Boolean) (ElapsedSeconds :type "Float (double-precision)") (TriggeredSeconds :type "Float (double-precision)") (InputAction :type "InputAction Object Reference" :default "/Game/Game/Blueprint/Input/Actions/IA_Down_Cross.IA_Down_Cross"))
  ;[1 1 1] Input
  (:`Started`
    (`self.PlayAnimMontage` "/Game/Game/Blueprint/Mesh/Animation/AM_Down.AM_Down")
    (set `self.InputIndex` 2)
    (`self.PlayAnimSound`)
    (if (not (`self.bIsInputBlock`))
      (goto _label))))

(event `StopTimer`
  ;[1 1 1] Timer
  (`KismetSystemLibrary.K2_ClearAndInvalidateTimerHandle` (stale `StartTimer` _returnvalue)))

(event `DisplayGameOver`
  ;[1 1 1] Timer
  (`WidgetLayoutLibrary.RemoveAllWidgets`)
  (bind _returnvalue (`|CreateWidget` "/Game/Game/UI/WBP_GameOver.WBP_GameOver_C" null self))
  (`UserWidget.AddToViewport` _returnvalue 0)
  (`AudioComponent.Stop` (`self.Music`)))

(event `StartTimer`
  ;[1 1 1] Timer
  (set `self.bIsTimerOn` true)
  (bind _returnvalue (`KismetSystemLibrary.K2_SetTimerDelegate` (delegate `Timer`) 0.01 true)))

(event `EnhancedInput|/Game/Game/Blueprint/Input/Actions/IA_Right_Circle`
  (params (ActionValue :type Boolean) (ElapsedSeconds :type "Float (double-precision)") (TriggeredSeconds :type "Float (double-precision)") (InputAction :type "InputAction Object Reference" :default "/Game/Game/Blueprint/Input/Actions/IA_Right_Circle.IA_Right_Circle"))
  ;[1 1 1] Input
  (:`Started`
    (`self.PlayAnimMontage` "/Game/Game/Blueprint/Mesh/Animation/AM_RIght.AM_RIght")
    (set `self.InputIndex` 3)
    (`self.PlayAnimSound`)
    (if (not (`self.bIsInputBlock`))
      (goto _label))))

(event `Timer`
  (bind _maxtimetofigure (`self.MaxTimeToFigure`))
  ;[1 1 1] Timer
  (bind _output_get (set `self.CurrentTimeToFigure` (- (`self.CurrentTimeToFigure`) 0.01)))
  (bind _returnvalue (`KismetMathLibrary.FClamp` _output_get 0.0 _maxtimetofigure))
  (`/Game/Game/UI/WBP_InGame.TimerBar` (`self.WBP_InGame`) (/ _returnvalue _maxtimetofigure))
  (if (== _returnvalue 0.0)
    (`/Engine/EditorBlueprintResources/StandardMacros.DoOnce` false :!label _label_2
      (:`Completed`
        (`/Game/Game/Blueprint/BP_Curtain.CloseCurtain` (`self.BP_Curtain`))
        (set `self.bIsLose` true)
        (`self.StopTimer`)))))

(event `StartGame`
  (`/Game/Game/Blueprint/BP_Curtain.OpenCurtain` (`self.BP_Curtain`) :!label _label_3)
  (bind _returnvalue (`|CreateWidget` "/Game/Game/UI/WBP_InGame.WBP_InGame_C" null self))
  (bind _output_get (set `self.WBP_InGame` _returnvalue))
  (`UserWidget.AddToViewport` _output_get 0)
  (`/Engine/EditorBlueprintResources/StandardMacros.IsValid` (`self.Music`)
    (:`Is Valid`
      _)
    (:`Is Not Valid`
      (bind _returnvalue_2 (`GameplayStatics.CreateSound2D` "/Game/Game/Sound/A_Musique_Fond.A_Musique_Fond" 0.05 1.0 0.0 null))
      (set `self.Music` _returnvalue_2)))
  (`AudioComponent.Play` (`self.Music`) 0.0)
  (`KismetSystemLibrary.Delay` 3.0)
  (set `self.bIsInputBlock` false)
  (`self.DefineNewFigure`)
  (`self.StartTimer`))

(event `EnhancedInput|/Game/Game/Blueprint/Input/Actions/IA_Up_Triangle`
  (params (ActionValue :type Boolean) (ElapsedSeconds :type "Float (double-precision)") (TriggeredSeconds :type "Float (double-precision)") (InputAction :type "InputAction Object Reference" :default "/Game/Game/Blueprint/Input/Actions/IA_Up_Triangle.IA_Up_Triangle"))
  ;[1 1 1] Input
  (:`Started`
    (`self.PlayAnimMontage` "/Game/Game/Blueprint/Mesh/Animation/AM_Up.AM_Up")
    (set `self.InputIndex` 4)
    (`self.PlayAnimSound`)
    (if (not (`self.bIsInputBlock`))
      (goto _label))))

(event `ResetTimer`
  ;[1 1 1] Timer
  (goto _label_2 :!via `Reset`))

(event `Replay`
  (`self.ResetAllVar`)
  (`WidgetLayoutLibrary.RemoveAllWidgets`)
  (goto _label_3))

(event `CheckCombo`
  (bind _returnvalue (- (`KismetArrayLibrary.Array_Length` (`self.CurrentFigurePlay`)) 1))
  ;[1 1 1] Check If The Combo Is Correct
  (for _index (range (+ _returnvalue 1))
    (if (== (`|GetArrayItem` (`self.RandomCombo`) _index) (`|GetArrayItem` (`self.CurrentFigurePlay`) _index))
      (if (and (== _returnvalue _index) (== (`KismetArrayLibrary.Array_Length` (`self.RandomCombo`)) (`KismetArrayLibrary.Array_Length` (`self.CurrentFigurePlay`))))
        (`/Engine/EditorBlueprintResources/StandardMacros.DoOnce` false :!label _label_4
          (:`Completed`
            (`self.ComboSucess`))))
      (else
        (`/Engine/EditorBlueprintResources/StandardMacros.DoOnce` false :!label _label_5
          (:`Completed`
            (`self.ComboFail`)))))))

(event `ComboSucess`
  (bind _difficulty (`self.Difficulty`))
  (bind _music (`self.Music`))
  ;[1 1 1] Check If The Combo Is Correct
  (set `self.bIsInputBlock` true)
  (bind _output_get (set `self.bIsSucess` true))
  (`self.UpdateTimer` _output_get)
  (`|PlayMontage` (`/Game/Game/Blueprint/BP_King.King` (`self.BP_King`)) "/Game/Game/Props/King/Anim/AM_Roi_Yey.AM_Roi_Yey"
    (:`then`
      (`GameplayStatics.PlaySoundAtLocation` "/Game/Game/Sound/King/A_KingGood.A_KingGood" (-600.0 0.0 0.0) (struct) 2.0 1.0 0.0 null null null null)
      (`NiagaraFunctionLibrary.SpawnSystemAtLocation` "/Game/Game/FX/Win/NS_SpirkleEffect.NS_SpirkleEffect" (- (`SceneComponent.K2_GetComponentLocation` (`self.Camera`)) (0.0 250.0 50.0)) (struct :`Roll` 80.0))
      (set `self.Score` (+ (`self.Score`) (* (* (`self.SucessScore`) (+ (`self.Streak`) 1)) (`self.Difficulty`)))))
    (:`OnCompleted`
      (bind _result (`/Engine/EditorBlueprintResources/StandardMacros.IncrementInt` (`self.Streak`))
        (:`  `
          (if (== _result (* (`self.Difficulty`) 3))
            (`/Engine/EditorBlueprintResources/StandardMacros.IncrementInt` (`self.Difficulty`)
              (:`  `
                _)))
          (`GameplayStatics.SetGlobalTimeDilation` (+ (* _difficulty 0.1) 0.9) :!label _label_6)
          (`/Engine/EditorBlueprintResources/StandardMacros.IsValid` _music
            (:`Is Valid`
              (`AudioComponent.SetPitchMultiplier` _music (+ (* _difficulty 0.05) 0.95)))
            (:`Is Not Valid`
              _))
          (`KismetSystemLibrary.Delay` 1.0)
          (if (`self.bIsTimerOn`)
            (set `self.bIsSucess` true)
            (`self.DefineNewFigure`)))))))

(event `ComboFail`
  ;[1 1 1] Check If The Combo Is Correct
  (set `self.bIsInputBlock` true)
  (bind _output_get (set `self.bIsSucess` false))
  (`self.UpdateTimer` _output_get)
  (`|PlayMontage` (`/Game/Game/Blueprint/BP_King.King` (`self.BP_King`)) "/Game/Game/Props/King/Anim/AM_Roi_Nooo.AM_Roi_Nooo"
    (:`then`
      (`GameplayStatics.PlaySoundAtLocation` "/Game/Game/Sound/King/A_KingBad.A_KingBad" (-600.0 0.0 0.0) (struct) 2.0 1.0 0.0 null null null null)
      (`GameplayStatics.PlaySoundAtLocation` "/Game/Game/Sound/Bouffon/A_Bouffon_Bad.A_Bouffon_Bad" (600.0 0.0 0.0) (struct) 0.4 1.0 0.0 null null null null))
    (:`OnCompleted`
      (set `self.Difficulty` 1 :!label _label_7)
      (set `self.Streak` 0)
      (goto _label_6))
    (:`OnInterrupted`
      (goto _label_7))))

(event `ResetCombo`
  ;[1 1 1] Check If The Combo Is Correct
  (`|ExecutionSequence`
    (:`then_0`
      (goto _label_4 :!via `Reset`))
    (:`then_1`
      (goto _label_5 :!via `Reset`))))

(event `self.ReceiveTick`
  (params (DeltaSeconds :type "Float (single-precision)"))
  ;[1 1 1] Check If The Combo Is Correct
  (`KismetSystemLibrary.PrintString` (`KismetStringLibrary.Conv_IntToString` (`self.Score`)) true true (struct :`G` 0.66 :`B` 1.0 :`A` 1.0) 0.0))

(event `DefineNewFigure`
  (bind _bp_saxopeople (`self.BP_SaxoPeople`))
  (bind _bp_bannier (`self.BP_Bannier`))
  (bind _bp_godhand (`self.BP_GodHand`))
  (bind _bp_king (`self.BP_King`))
  (bind _bp_king_2 (`self.BP_King`))
  ;[1 1 1] Define A Random Combo Base On Difficulty
  (if (not (`self.bIsLose`))
    (`KismetArrayLibrary.Array_Clear` (`self.CurrentFigurePlay`))
    (`KismetArrayLibrary.Array_Clear` (`self.RandomCombo`))
    (for _ (range (+ (+ (`self.Difficulty`) 1) 1))
      (`KismetArrayLibrary.Array_Add` (`self.RandomCombo`) (`KismetMathLibrary.RandomIntegerInRange` 1 4)))
    (`|ExecutionSequence`
      (:`then_0`
        (set `self.bIsInputBlock` false)
        (`self.ResetCombo`))
      (:`then_1`
        (if (not (== (`self.IndexTuto`) 0))
          (`/Engine/EditorBlueprintResources/StandardMacros.DecrementInt` (`self.IndexTuto`)
            (:`  `
              (`/Engine/EditorBlueprintResources/StandardMacros.IsValid` _bp_king :!label _label_8
                (:`Is Valid`
                  (`/Game/Game/Blueprint/BP_King.KingTalk` _bp_king)
                  (set `self.SucessScore` 15)))))
          (else
            (bind _sumofvalue (`self.SumValue`))
            (bind _randomindex (`self.DetermineIndex` (`KismetMathLibrary.RandomFloatInRange` 0.0 _sumofvalue)))
            (switch `int` _randomindex
              (:`0`
                (goto _label_8))
              (:`1`
                (`/Engine/EditorBlueprintResources/StandardMacros.IsValid` _bp_king_2
                  (:`Is Valid`
                    (`/Game/Game/Blueprint/BP_King.KingSign` _bp_king_2)
                    (set `self.SucessScore` 10))))
              (:`2`
                (`/Engine/EditorBlueprintResources/StandardMacros.IsValid` _bp_bannier
                  (:`Is Valid`
                    (`/Game/Game/Blueprint/BP_Bannier.BeginCombo` _bp_bannier)
                    (set `self.SucessScore` 30))))
              (:`3`
                (`/Engine/EditorBlueprintResources/StandardMacros.IsValid` _bp_saxopeople
                  (:`Is Valid`
                    (`/Game/Game/Blueprint/Bp_SaxoPeople.BeginCombo` _bp_saxopeople)
                    (set `self.SucessScore` 50))))
              (:`4`
                (`/Engine/EditorBlueprintResources/StandardMacros.IsValid` _bp_godhand
                  (:`Is Valid`
                    (`/Game/Game/Blueprint/BP_GodHand.BeginCombo` _bp_godhand)
                    (set `self.SucessScore` 100)))))))))))

(event `ResetAllVar`
  (set `self.Score` 0)
  (set `self.SucessScore` 10)
  (set `self.bIsLose` false)
  (set `self.bIsInputBlock` true)
  (`KismetArrayLibrary.Array_Clear` (`self.CurrentFigurePlay`))
  (`KismetArrayLibrary.Array_Clear` (`self.RandomCombo`))
  (set `self.Difficulty` 1)
  (set `self.Streak` 0)
  (set `self.IndexTuto` 3)
  (set `self.MaxTimeToFigure` 50.0)
  (set `self.CurrentTimeToFigure` 50.0)
  (`self.ResetTimer`)
  (set `self.bIsSucess` true)
  (set `self.InputIndex` 0)
  (set `self.bIsTimerOn` false))

(fn `DetermineIndex`
  (params (RandomValue :type "Float (double-precision)"))
  (returns (RandomIndex :type Integer))
  (locals (LocalSum :type "Float (double-precision)"))
  (bind _keys (`BlueprintMapLibrary.Map_Keys` (`self.WeightValue`)))
  (for (_array_element _array_index) _keys
    (bind _output_get (set `local.LocalSum` (+ _array_element (`local.LocalSum`))))
    (if (>= _output_get (`local.RandomValue`))
      (break)))
  (return _array_index))

(fn `SumValue`
  (returns (SumOfValue :type "Float (double-precision)"))
  (locals (LocalSum :type "Float (double-precision)"))
  (bind _localsum (`local.LocalSum`))
  (bind _keys (`BlueprintMapLibrary.Map_Keys` (`self.WeightValue`)))
  (for _array_element _keys
    (set `local.LocalSum` (+ _array_element _localsum)))
  (return _localsum))

(fn `UpdateTimer`
  (params (bIsSucess :type Boolean))
  (set `self.CurrentTimeToFigure` (`KismetMathLibrary.FClamp` (+ (`self.CurrentTimeToFigure`) (select `bool` bIsSucess :`false` (* (/ (`self.MaxTimeToFigure`) 2.0) -1.0) :`true` (/ (`self.MaxTimeToFigure`) 4.0))) 0.0 (`self.MaxTimeToFigure`)))
  (return))

(fn `UserConstructionScript`)