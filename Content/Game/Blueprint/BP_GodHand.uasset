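; BP_GodHand is a hand that descends into the stage to show the player's BP_Bouffon random direction combo.
; BeginCombo plays a timeline that lowers the plane from its initial location.
; Direction and ShowNext then step through RandomCombo with delays, swapping a dynamic material texture between arrow-direction hand signs and a neutral pose.
; After the last sign, Retreat reverses the timeline to raise the hand.
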(event `self.ReceiveBeginPlay`
  ;[1 1 1] Set Initial Variable
  (set `self.InitialLocation` (`SceneComponent.K2_GetComponentLocation` (`self.Plane`)))
  (bind _asbp_bouffon (cast `/Game/Game/Blueprint/BP_Bouffon` (`GameplayStatics.GetPlayerCharacter` 0)))
  (set `self.BP_Bouffon` _asbp_bouffon)
  (bind _returnvalue (`PrimitiveComponent.CreateDynamicMaterialInstance` (`self.Plane`) 0 null "None"))
  (set `self.Material` _returnvalue))

(event `StartMove`
  ;[1 1 1] Move The God Hand In The Stage
  (set `self.bIsFinishPlaying` false)
  (`TimelineComponent.SetPlayRate` (`self.Move`) 0.8)
  (bind (_direction _alpha) (`Timeline|Move` :!via `PlayFromStart` :!label _label)
    (:`Update`
      (`SceneComponent.K2_SetWorldLocation` (`self.Plane`) (`|EaseFunction` "Linear" _alpha (`self.InitialLocation`) (`KismetMathLibrary.MakeVector` (.x (`self.InitialLocation`)) (.y (`self.InitialLocation`)) (- (.z (`self.InitialLocation`)) (`self.Distance`)))) false false))
    (:`Finished`
      (if (not (`self.bIsFinishPlaying`))
        (`self.Direction`)))))

(event `Retreat`
  ;[1 1 1] Move The God Hand In The Stage
  (set `self.bIsFinishPlaying` true)
  (goto _label :!via `ReverseFromEnd`))

(event `BeginCombo`
  (set `self.CurrentIndex` 0)
  (`MaterialInstanceDynamic.SetTextureParameterValue` (`self.Material`) "HandSign" "/Game/Game/Props/GodHand/T_Hand_Neutral.T_Hand_Neutral")
  (`self.StartMove`))

(event `Direction`
  (bind _material (`self.Material`))
  (switch `int` (`|GetArrayItem` (`/Game/Game/Blueprint/BP_Bouffon.RandomCombo` (`self.BP_Bouffon`)) (`self.CurrentIndex`))
    (:`1`
      (`MaterialInstanceDynamic.SetTextureParameterValue` _material "HandSign" "/Game/Game/Props/GodHand/T_Hand_Left.T_Hand_Left"))
    (:`2`
      (`MaterialInstanceDynamic.SetTextureParameterValue` _material "HandSign" "/Game/Game/Props/GodHand/T_Hand_Down.T_Hand_Down"))
    (:`3`
      (`MaterialInstanceDynamic.SetTextureParameterValue` _material "HandSign" "/Game/Game/Props/GodHand/T_Hand_Right.T_Hand_Right"))
    (:`4`
      (`MaterialInstanceDynamic.SetTextureParameterValue` _material "HandSign" "/Game/Game/Props/GodHand/T_Hand_Up.T_Hand_Up")))
  (`self.ShowNext`))

(event `ShowNext`
  (bind _currentindex (`self.CurrentIndex`))
  (`KismetSystemLibrary.Delay` 0.2)
  (if (== (- (`KismetArrayLibrary.Array_Length` (`/Game/Game/Blueprint/BP_Bouffon.RandomCombo` (`self.BP_Bouffon`))) 1) _currentindex)
    (set `self.CurrentIndex` 0)
    (`KismetSystemLibrary.Delay` 0.5)
    (`self.Retreat`)
    (else
      (`/Engine/EditorBlueprintResources/StandardMacros.IncrementInt` _currentindex
        (:`  `
          (`MaterialInstanceDynamic.SetTextureParameterValue` (`self.Material`) "HandSign" "/Game/Game/Props/GodHand/T_Hand_Neutral.T_Hand_Neutral")
          (`KismetSystemLibrary.Delay` 0.2)
          (`self.Direction`))))))

(fn `UserConstructionScript`)