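; BP_Curtain is a stage curtain actor that frames the start and end of a game round for the BP_Bouffon player character, which it caches on BeginPlay.
; OpenCurtain plays the curtain animation and opening sound while immediately telling the player to start the game.
; CloseCurtain plays a montage from a one-second offset with a closing sound, then has the player display game over once the montage completes.
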(event `self.ReceiveBeginPlay`
  (bind _asbp_bouffon (cast `/Game/Game/Blueprint/BP_Bouffon` (`GameplayStatics.GetPlayerCharacter` 0)))
  (set `self.BP_Bouffon` _asbp_bouffon))

(event `OpenCurtain`
  (`SkeletalMeshComponent.PlayAnimation` (`self.SkeletalMesh`) "/Game/Game/Props/Curtain/A_Curtain.A_Curtain" false)
  (`/Game/Game/Blueprint/BP_Bouffon.StartGame` (`self.BP_Bouffon`))
  (`GameplayStatics.PlaySound2D` "/Game/Game/Sound/A_CurtainOpen.A_CurtainOpen" 0.7 1.0 0.0 null null false))

(event `CloseCurtain`
  (`|PlayMontage` (`self.SkeletalMesh`) "/Game/Game/Props/Curtain/AM_Curtain.AM_Curtain" 1.0 1.0
    (:`then`
      (`GameplayStatics.PlaySound2D` "/Game/Game/Sound/A_CurtainClose.A_CurtainClose" 0.7 1.0 0.0 null null false))
    (:`OnCompleted`
      (`/Game/Game/Blueprint/BP_Bouffon.DisplayGameOver` (`self.BP_Bouffon`)))))

(fn `UserConstructionScript`)