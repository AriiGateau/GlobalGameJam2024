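; BP_Test is a test Blueprint that hangs a Cable component's end on a Cylinder component.
; The construction script sets that attachment, and BeginPlay applies it again.
; BeginPlay then shifts the cylinder by a random offset along world X, keeping Y and Z, so the cable's end point varies each play.
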(event `self.ReceiveBeginPlay`
  (bind _cylinder (`self.Cylinder`))
  (bind (_returnvalue_x _returnvalue_y _returnvalue_z) (`KismetMathLibrary.BreakVector` (`SceneComponent.K2_GetComponentLocation` _cylinder)))
  (`CableComponent.SetAttachEndToComponent` (`self.Cable`) (`self.Cylinder`) "None")
  (`SceneComponent.K2_SetWorldLocation` _cylinder (`KismetMathLibrary.MakeVector` (+ _returnvalue_x (`KismetMathLibrary.RandomFloatInRange` -100.0 100.0)) _returnvalue_y _returnvalue_z) false false))

(fn `UserConstructionScript`
  (`CableComponent.SetAttachEndToComponent` (`self.Cable`) (`self.Cylinder`) "None"))